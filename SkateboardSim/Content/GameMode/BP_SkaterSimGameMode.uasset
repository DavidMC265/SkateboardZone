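; Game mode for a skateboarding game that runs a countdown in which the player must reach waypoint and point targets.
; BeginPlay creates the HUD and locks character input briefly while intro text shows.
; Tick uses a one-second Delay as a throttle to decrement and display the timer.
; If time hits zero with either target unmet, it shows the lose screen, disables input and reveals the cursor.
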(event `self.ReceiveBeginPlay`
  ;[0 0 0] BeginPlay
  (bind _asbp_skate_board_character (cast `/Game/Characters/SkateboardCharacter/BP_SkateBoardCharacter` (`GameplayStatics.GetPlayerCharacter` 0)))
  (set `self.SkateboardCharacter` _asbp_skate_board_character)
  (bind _returnvalue (`|CreateWidget` "/Game/UI/WBP_PlayerWidget.WBP_PlayerWidget_C" (`GameplayStatics.GetPlayerController` 0)))
  (bind _output_get (set `self.Player Widget` _returnvalue))
  (`UserWidget.AddToViewport` _output_get 0)
  (`TextBlock.SetText` (`/Game/UI/WBP_PlayerWidget.Countdown` (`self.Player Widget`)) (`KismetTextLibrary.Conv_IntToText` (`self.CountdownTime`)))
  (set `self.GameHasBegun` true)
  (`self.HideTextsAfterDelay`))

(event `self.ReceiveTick`
  (params (DeltaSeconds :type "Float (single-precision)"))
  ;[0 0 0] Countdown Timer UI functionality
  (if (`self.GameHasBegun`)
    (`/Engine/EditorBlueprintResources/StandardMacros.IsValid` (`self.Player Widget`)
      (:`Is Valid`
        (`/Engine/EditorBlueprintResources/StandardMacros.IsValid` (`self.SkateboardCharacter`)
          (:`Is Valid`
            (`KismetSystemLibrary.Delay` 1.0)
            (bind _output_get (set `self.CountdownTime` (- (`self.CountdownTime`) 1)))
            (if (and (== (`self.CountdownTime`) 0) (or (< (`self.UpdatedWaypoints`) (`self.WaypointsToCollect`)) (< (`self.UpdatedPoints`) (`self.PointsToAquire`))))
              (`self.HandlePlayerLoose`)
              (else
                (`TextBlock.SetText` (`/Game/UI/WBP_PlayerWidget.Countdown` (`self.Player Widget`)) (`KismetTextLibrary.Conv_IntToText` _output_get))))))))))

(fn `HandlePlayerLoose`
  (bind _returnvalue (`GameplayStatics.GetPlayerController` 0))
  (`TextBlock.SetText` (`/Game/UI/WBP_PlayerWidget.Countdown` (`self.Player Widget`)) (`KismetTextLibrary.Conv_IntToText` 0))
  (bind _returnvalue_2 (`|CreateWidget` "/Game/UI/WBP_LooseScreen.WBP_LooseScreen_C" (`GameplayStatics.GetPlayerController` 0)))
  (`UserWidget.AddToViewport` _returnvalue_2 10)
  (`self.DisableInput` _returnvalue _returnvalue)
  (set `PlayerController.bShowMouseCursor` true _returnvalue))

(fn `UserConstructionScript`)