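; BP_building_adver_01 is a configurable neon advertising prop for buildings, with a mesh and two point lights.
; Its construction script picks the Neon mesh from an array by ObjectId.
; A shared Color index selects both the neon material and the matching color for both lights, which also receive the Intensity value.
; The event graph holds only disabled placeholder events, so the prop has no runtime logic.
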(fn `UserConstructionScript`
  (bind _neon (`self.neon`))
  (bind _color (`self.color`))
  (bind _pointlight1 (`self.PointLight1`))
  (`StaticMeshComponent.SetStaticMesh` _neon (`|GetArrayItem` (`self.meshes`) (`self.object_id`)))
  (`PrimitiveComponent.SetMaterial` _neon 0 (`|GetArrayItem` (`self.materials`) _color))
  (`LightComponent.SetLightColor` _pointlight1 (`|GetArrayItem` (`self.Light Color`) _color) true)
  (`LightComponent.SetLightColor` (`self.PointLight2`) (`|GetArrayItem` (`self.Light Color`) _color) true)
  (`LightComponent.SetIntensity` _pointlight1 (`self.Intensity`))
  (`LightComponent.SetIntensity` (`self.PointLight2`) (`self.Intensity`)))