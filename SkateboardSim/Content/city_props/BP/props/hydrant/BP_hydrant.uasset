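; Fire hydrant city prop Blueprint that sprays water when either its left or right side is hit.
; Each side has its own hit proxy, whose first hit toggles off that side's destructible component and activates its water splash and flow cue.
; A DoOnce makes each side trigger only once, and its water effects shut off after a fixed delay.
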(event `self.ReceiveBeginPlay`)

(event `self.hit_proxy_r.OnComponentHit`
  (params (HitComponent :type "PrimitiveComponent Object Reference") (OtherActor :type "Actor Object Reference") (OtherComp :type "PrimitiveComponent Object Reference") (NormalImpulse :type "Vector Structure") (Hit :type "HitResult Structure (by ref)"))
  (`/Engine/EditorBlueprintResources/StandardMacros.DoOnce` false
    (:`Completed`
      (`ActorComponent.SetActive` (`self.water_splash_r`) true true)
      (`ActorComponent.SetActive` (`self.water_flow_cue_r`) true true)
      (`SceneComponent.ToggleVisibility` (`self.Destructible_r`) false)
      (`KismetSystemLibrary.Delay` 15.0)
      (`ActorComponent.SetActive` (`self.water_splash_r`) false false)
      (`ActorComponent.SetActive` (`self.water_flow_cue_r`) false false))))

(event `self.hit_proxy_l.OnComponentHit`
  (params (HitComponent :type "PrimitiveComponent Object Reference") (OtherActor :type "Actor Object Reference") (OtherComp :type "PrimitiveComponent Object Reference") (NormalImpulse :type "Vector Structure") (Hit :type "HitResult Structure (by ref)"))
  (`/Engine/EditorBlueprintResources/StandardMacros.DoOnce` false
    (:`Completed`
      (`ActorComponent.SetActive` (`self.water_splash_l`) true true)
      (`ActorComponent.SetActive` (`self.water_flow_cue_l`) true true)
      (`SceneComponent.ToggleVisibility` (`self.Destructible_l`) false)
      (`KismetSystemLibrary.Delay` 15.0)
      (`ActorComponent.SetActive` (`self.water_splash_l`) false false)
      (`ActorComponent.SetActive` (`self.water_flow_cue_l`) false false))))

(fn `UserConstructionScript`)